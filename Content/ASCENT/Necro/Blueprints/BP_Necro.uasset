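; BP_Necro is a Necro pawn Blueprint that is an early or debug stub with little working behavior.
; On BeginPlay it activates its Camera, and every Tick it prints a "Hello" debug string.
; Unconnected nodes sketch forward/right movement, a PointLight offset from the actor, and yaw rotation toward that offset, but none execute and the offsets multiply to zero.
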(event Collision|EventActorBeginOverlap
  (params (OtherActor :type Actor%20Object%20Reference)))

(event EventBeginPlay
  (Components|Activation|Activate (Variables|Default|GetCamera) false))

(event EventTick
  (params (DeltaSeconds :type Float%20%28single-precision%29))
  (Development|PrintString "Hello"))

(fn ConstructionScript)